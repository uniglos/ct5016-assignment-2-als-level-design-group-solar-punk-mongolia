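; BP_Console is an interactable console where the player is prompted to plant a bomb.
; On BeginPlay it finds BP_Player and binds OpenDoor to its Interact dispatcher.
; The Trigger overlap tracks whether the player is in range and updates or collapses the player's InteractWidget prompt.
; Interacting in range sets Activated, prints "Kaboom" and hides the prompt; despite its name, OpenDoor moves no door.
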(event OnComponentBeginOverlap(Trigger)
  (params (OverlappedComponent :type Primitive%20Component%20Object%20Reference) (OtherActor :type Actor%20Object%20Reference) (OtherComp :type Primitive%20Component%20Object%20Reference) (OtherBodyIndex :type Integer) (bFromSweep :type Boolean) (SweepResult :type Hit%20Result%20Structure%20%28by%20ref%29))
  (if (== OtherActor (Game|Player|GetPlayerPawn 0))
    (Development|PrintString "In Trigger")
    (Variables|Default|SetInTrigger? true)
    (if (not (Variables|Default|GetActivated?))
      (Default|ChangeText (Variables|/Game/Blueprints/BP_Player.BP_Player_C|GetInteractWidget (Variables|Default|GetPlayer)) "Press 'K' to Plant Bomb"))))

(event OnComponentEndOverlap(Trigger)
  (params (OverlappedComponent :type Primitive%20Component%20Object%20Reference) (OtherActor :type Actor%20Object%20Reference) (OtherComp :type Primitive%20Component%20Object%20Reference) (OtherBodyIndex :type Integer))
  (if (== OtherActor (Game|Player|GetPlayerPawn 0))
    (Development|PrintString "Left Trigger")
    (Variables|Default|SetInTrigger? false)
    (Widget|SetVisibility (Variables|/Game/Blueprints/BP_Player.BP_Player_C|GetInteractWidget (Variables|Default|GetPlayer)) "Collapsed")))

(event Custom|OpenDoor
  (if (Variables|Default|GetInTrigger?)
    (Development|PrintString "Kaboom")
    (Variables|Default|SetActivated? true)
    (Widget|SetVisibility (Variables|/Game/Blueprints/BP_Player.BP_Player_C|GetInteractWidget (Variables|Default|GetPlayer)) "Collapsed")))

(event EventBeginPlay
  (bind _returnvalue (Actor|GetActorOfClass "/Game/Blueprints/BP_Player.BP_Player_C"))
  (bind _output_get (Variables|Default|SetPlayer _returnvalue))
  (EventDispatchers|AssignInteract _output_get (delegate Custom|OpenDoor)))

(fn ConstructionScript)